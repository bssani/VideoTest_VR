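; Stereo 3D media player actor that plays video on a flat, curved, 180 or 360 dome screen mesh.
; The construction script creates a dynamic instance of M_Stereo3D and sets the screen mesh.
; Events control MediaPlayer playback, seeking and volume, while material parameters switch projection and stereo layout and adjust image settings.
; Tick caches the current playback time once media loads; aspect ratio scaling applies only to flat screens.
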(event Custom|ChangeScreenType
  (params (ScreenType :type E_ScreenType%20Enum :default "NewEnumerator0"))
  (bind _screenmesh (Variables|Default|GetScreenMesh))
  ;[0 0 0] Change Screen
  (switch Utilities|FlowControl|Switch|SwitchonE_ScreenType ScreenType
    (:NewEnumerator0
      (Components|StaticMesh|SetStaticMesh _screenmesh "/Game/VR_MediaPlayer/Static_Mesh/SM_FlatScreen.SM_FlatScreen")
      (Transformation|SetRelativeScale3D (Variables|Default|GetScreenMesh) "1.000000,1.000000,1.000000" :!label _label))
    (:NewEnumerator1
      (Components|StaticMesh|SetStaticMesh _screenmesh "/Game/VR_MediaPlayer/Static_Mesh/SM_CurveScreen.SM_CurveScreen")
      (goto _label))
    (:NewEnumerator2
      (Components|StaticMesh|SetStaticMesh _screenmesh "/Game/VR_MediaPlayer/Static_Mesh/SM_180Dome.SM_180Dome")
      (Transformation|SetRelativeScale3D (Variables|Default|GetScreenMesh) "300.000000,300.000000,300.000000" :!label _label_2))
    (:NewEnumerator3
      (Components|StaticMesh|SetStaticMesh _screenmesh "/Game/VR_MediaPlayer/Static_Mesh/SM_360Dome.SM_360Dome")
      (goto _label_2))))

(event Custom|ChangeProjectionType
  (params (ProjectionType :type E_ProjectionType%20Enum :default "NewEnumerator0"))
  (bind _screenmaterial (Variables|Default|GetScreenMaterial))
  ;[0 0 0] 2D/3D switch
  (switch Utilities|FlowControl|Switch|SwitchonE_ProjectionType ProjectionType
    (:NewEnumerator0
      (Rendering|Material|SetScalarParameterValue _screenmaterial "2Dprojection" 1.0 :!class /Script/Engine.MaterialInstanceDynamic))
    (:NewEnumerator1
      (Rendering|Material|SetScalarParameterValue _screenmaterial "2Dprojection" 0.0 :!class /Script/Engine.MaterialInstanceDynamic))))

(event Custom|PauseMedia
  ;[0 0 0] Star/Play/Pause/seek media
  (Sequencer|Player|Pause (Variables|Default|GetMediaPlayer)))

(event Custom|OnSeekCompleted_Event
  ;[0 0 0] Star/Play/Pause/seek media
  (Media|MediaPlayer|Play (Variables|Default|GetMediaPlayer) :!class /Script/MediaAssets.MediaPlayer))

(event Custom|UpdatePlayTime
  (bind _mediaplayer (Variables|Default|GetMediaPlayer))
  (bind _returnvalue (Class|MediaPlayer|GetTimeStamp _mediaplayer))
  (bind _time (Variables|/Script/MediaAssets.MediaTimeStampInfo|GetTime _returnvalue))
  ;[0 0 0] UpdateTimeline
  (if (Variables|Default|GetMediaLoaded)
    (Variables|Default|SetCurrentHours (.hours _time))
    (Variables|Default|SetCurrentMinutes (.minutes _time))
    (Variables|Default|SetCurrentSeconds (.seconds _time))
    (Variables|Default|SetCurrentMilliseconds (Class|KismetMathLibrary|GetTotalMilliseconds (Class|MediaPlayer|GetTime _mediaplayer)))))

(event Custom|Seek
  (params (Time :type Timespan%20Structure%20%28by%20ref%29))
  (bind _mediaplayer (Variables|Default|GetMediaPlayer))
  ;[0 0 0] Star/Play/Pause/seek media
  (Sequencer|Player|Pause _mediaplayer)
  (Media|MediaPlayer|Seek _mediaplayer Time)
  (EventDispatchers|AssignOnSeekCompleted _mediaplayer (delegate Custom|OnSeekCompleted_Event)))

(event Custom|ChangeVolume
  (params (Volume :type Float%20%28double-precision%29))
  ;[0 0 0] Set Audio level
  (Class|MediaPlayer|SetNativeVolume (Variables|Default|GetMediaPlayer) Volume))

(event Custom|ChangeStereoType
  (params (StereoMode :type E_StereoMode%20Enum :default "NewEnumerator0"))
  (bind _screenmaterial (Variables|Default|GetScreenMaterial))
  ;[0 0 0] Stereo Setting
  (switch Utilities|FlowControl|Switch|SwitchonE_StereoMode StereoMode
    (:NewEnumerator0
      (Rendering|Material|SetScalarParameterValue _screenmaterial "SBS" 1.0 :!class /Script/Engine.MaterialInstanceDynamic))
    (:NewEnumerator1
      (Rendering|Material|SetScalarParameterValue _screenmaterial "SBS" 0.0 :!class /Script/Engine.MaterialInstanceDynamic))
    (:NewEnumerator2
      (Rendering|Material|SetScalarParameterValue _screenmaterial "Stereo" 0.0 :!class /Script/Engine.MaterialInstanceDynamic))
    (:NewEnumerator3
      (Rendering|Material|SetScalarParameterValue _screenmaterial "Stereo" 1.0 :!class /Script/Engine.MaterialInstanceDynamic))))

(event Custom|ChangeBrightness
  (params (Brightness :type Float%20%28double-precision%29))
  ;[0 0 0] ImageControl
  (Rendering|Material|SetScalarParameterValue (Variables|Default|GetScreenMaterial) "Brightness" Brightness :!class /Script/Engine.MaterialInstanceDynamic))

(event Custom|ChangeSaturation
  (params (Saturation :type Float%20%28double-precision%29))
  ;[0 0 0] ImageControl
  (Rendering|Material|SetScalarParameterValue (Variables|Default|GetScreenMaterial) "Saturation" Saturation :!class /Script/Engine.MaterialInstanceDynamic))

(event Custom|ChangeContrast
  (params (Contrast :type Float%20%28double-precision%29))
  ;[0 0 0] ImageControl
  (Rendering|Material|SetScalarParameterValue (Variables|Default|GetScreenMaterial) "Contrast" Contrast :!class /Script/Engine.MaterialInstanceDynamic))

(event Custom|ChangeAspectRatio
  (params (AspectRatio :type Float%20%28double-precision%29))
  (bind _screenmesh (Variables|Default|GetScreenMesh))
  ;[0 0 0] Set Aspect Ratio
  (if (Utilities|Enum|Equal(Enum) (Variables|Default|GetScreenType) "NewEnumerator0")
    (Transformation|SetRelativeScale3D _screenmesh "1.000000,1.000000,1.000000")
    (Transformation|SetRelativeScale3D _screenmesh (* (Variables|/Script/Engine.SceneComponent|GetRelativeScale3D _screenmesh) (Math|Vector|MakeVector AspectRatio 1.0 1.0)))
    (else
      (Transformation|SetRelativeScale3D _screenmesh "1.000000,1.000000,1.000000"))))

(event Custom|StartMedia
  (params (MediaSource :type Media%20Source%20Object%20Reference) (MediaTexture :type Texture%20Object%20Reference))
  (bind _mediaplayer (Variables|Default|GetMediaPlayer))
  ;[0 0 0] Star/Play/Pause/seek media
  (Rendering|Material|SetTextureParameterValue (Variables|Default|GetScreenMaterial) "InputMedia" MediaTexture)
  (Media|MediaPlayer|OpenSource _mediaplayer MediaSource)
  (Media|MediaPlayer|BindEventtoOnMediaOpened _mediaplayer (delegate Custom|OnMediaLoad)))

(event Custom|OnMediaLoad
  (params (OpenedUrl :type String))
  (bind _mediaplayer (Variables|Default|GetMediaPlayer))
  (bind _returnvalue (Media|MediaPlayer|GetDuration _mediaplayer))
  ;[0 0 0] Star/Play/Pause/seek media
  (Variables|Default|SetHours (.hours _returnvalue))
  (Variables|Default|SetMinutes (.minutes _returnvalue))
  (Variables|Default|SetSeconds (.seconds _returnvalue))
  (Variables|Default|SetMediaLengthMilliseconds (Class|KismetMathLibrary|GetTotalMilliseconds (Media|MediaPlayer|GetDuration _mediaplayer)))
  (Variables|Default|SetMediaLoaded true))

(event Custom|ResumeMedia
  ;[0 0 0] Star/Play/Pause/seek media
  (Media|MediaPlayer|Play (Variables|Default|GetMediaPlayer) :!class /Script/MediaAssets.MediaPlayer))

(event EventTick
  (params (DeltaSeconds :type Float%20%28single-precision%29))
  (CallFunction|UpdatePlayTime))

(fn ConstructionScript
  (bind _screenmesh (Variables|Default|GetScreenMesh))
  (bind _returnvalue (Rendering|Material|CreateDynamicMaterialInstance (Variables|Default|GetScreenMesh) 0 "/Game/VR_MediaPlayer/Materials/M_Stereo3D.M_Stereo3D" "None" :!class /Script/Engine.PrimitiveComponent))
  (Variables|Default|SetScreenMaterial _returnvalue)
  (switch Utilities|FlowControl|Switch|SwitchonE_ScreenType (Variables|Default|GetScreenType)
    (:NewEnumerator0
      (Components|StaticMesh|SetStaticMesh _screenmesh "/Game/VR_MediaPlayer/Static_Mesh/SM_FlatScreen.SM_FlatScreen")
      (Transformation|SetRelativeScale3D (Variables|Default|GetScreenMesh) "1.000000,1.000000,1.000000" :!label _label))
    (:NewEnumerator1
      (Components|StaticMesh|SetStaticMesh _screenmesh "/Game/VR_MediaPlayer/Static_Mesh/SM_CurveScreen.SM_CurveScreen")
      (goto _label))
    (:NewEnumerator2
      (Components|StaticMesh|SetStaticMesh _screenmesh "/Game/VR_MediaPlayer/Static_Mesh/SM_180Dome.SM_180Dome")
      (Transformation|SetRelativeScale3D (Variables|Default|GetScreenMesh) "300.000000,300.000000,300.000000" :!label _label_2))
    (:NewEnumerator3
      (Components|StaticMesh|SetStaticMesh _screenmesh "/Game/VR_MediaPlayer/Static_Mesh/SM_360Dome.SM_360Dome")
      (goto _label_2))))